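; Patrolling NPC that acts as a light source for the player's light detection.
; On BeginPlay its AI controller runs the BT_Patrol behavior tree.
; Capsule begin and end overlaps with the Sevarog player character call PassedIntoLight and PassedOutofLight on BP_UnseenPlayerController, passing the NPC itself.
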(event OnComponentBeginOverlap(Capsule)
  (params (OverlappedComponent :type Primitive%20Component%20Object%20Reference) (OtherActor :type Actor%20Object%20Reference) (OtherComp :type Primitive%20Component%20Object%20Reference) (OtherBodyIndex :type Integer) (bFromSweep :type Boolean) (SweepResult :type Hit%20Result%20Structure%20%28by%20ref%29))
  (bind _assevarog_player_character (Utilities|Casting|CastToSevarogPlayerCharacter OtherActor))
  (bind _asbp_unseen_player_controller (Utilities|Casting|CastToBP_UnseenPlayerController (Pawn|GetController _assevarog_player_character)))
  (Default|PassedIntoLight _asbp_unseen_player_controller self))

(event OnComponentEndOverlap(Capsule)
  (params (OverlappedComponent :type Primitive%20Component%20Object%20Reference) (OtherActor :type Actor%20Object%20Reference) (OtherComp :type Primitive%20Component%20Object%20Reference) (OtherBodyIndex :type Integer))
  (bind _assevarog_player_character (Utilities|Casting|CastToSevarogPlayerCharacter OtherActor))
  (bind _asbp_unseen_player_controller (Utilities|Casting|CastToBP_UnseenPlayerController (Pawn|GetController _assevarog_player_character)))
  (Default|PassedOutofLight _asbp_unseen_player_controller self))

(event EventBeginPlay
  (AI|RunBehaviorTree (AI|GetAIController self) "/Game/Project/BluePrints/AI/Patrol/BT_Patrol.BT_Patrol"))

(fn ConstructionScript)