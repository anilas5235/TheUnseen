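; BP_SoulShard is a collectable pickup that bobs and spins until the Severog player character touches it.
; On BeginPlay it registers itself with the Unseen player controller's collectable count and picks a random phase offset.
; Tick moves the sphere on a sine wave and yaws it, with the offset varying the bob between shards.
; On overlap it reports collection to that controller and destroys itself.
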(event OnComponentBeginOverlap(Coll)
  (params (OverlappedComponent :type Primitive%20Component%20Object%20Reference) (OtherActor :type Actor%20Object%20Reference) (OtherComp :type Primitive%20Component%20Object%20Reference) (OtherBodyIndex :type Integer) (bFromSweep :type Boolean) (SweepResult :type Hit%20Result%20Structure%20%28by%20ref%29))
  ;[1 1 1] Overlap
  (bind _assevarog_player_character (Utilities|Casting|CastToSevarogPlayerCharacter OtherActor))
  (bind _asbp_unseen_player_controller (Utilities|Casting|CastToBP_UnseenPlayerController (Pawn|GetController _assevarog_player_character)))
  (Default|Collected _asbp_unseen_player_controller "NewEnumerator0")
  (Actor|DestroyActor))

(event EventTick
  (params (DeltaSeconds :type Float%20%28single-precision%29))
  (bind _sphere (Variables|Default|GetSphere))
  ;[1 1 1] Tick
  (Transformation|SetRelativeLocation _sphere (Math|Vector|MakeVector 0.0 0.0 (* (Math|Trig|Sin(Radians) (+ (* (Utilities|Time|GetGameTimeinSeconds) (Variables|Default|GetUpDownFrequenz)) (Variables|Default|GetRandomTimeOffset))) (Variables|Default|GetUpDownMultiplier))) false true)
  (Transformation|AddRelativeRotation _sphere (Math|Rotator|MakeRotator 0.0 0.0 (* DeltaSeconds (Variables|Default|GetRotationRate))) false false))

(event EventBeginPlay
  ;[1 1 1] OnBegin
  (bind _asbp_unseen_player_controller (CallFunction|TryGetUnseenPlayerController))
  (Default|AddNumberOfCollectable _asbp_unseen_player_controller "NewEnumerator0")
  (Variables|Default|SetRandomTimeOffset (Math|Float|MultiplybyPi (Math|Random|RandomFloat))))

(fn ConstructionScript)