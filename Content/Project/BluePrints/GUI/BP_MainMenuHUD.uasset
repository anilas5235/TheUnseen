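; Main menu HUD that creates a set of menu widgets and controls which one is visible.
; On BeginPlay it instantiates each class in WidgetsClasses into the viewport and the Widgets array, collapsed, then calls SwitchToWidget for the first.
; SwitchToWidget collapses the current widget if its index is valid; only otherwise does it store and show the requested index.
; Its guard skips only a valid index that is already current.
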(event EventBeginPlay
  (for (_array_element _array_index) (Variables|Default|GetWidgetsClasses)
    (bind _returnvalue (UserInterface|CreateWidget _array_element))
    (UserInterface|Viewport|AddtoViewport _returnvalue 0)
    (Utilities|Array|SetArrayElem (Variables|Default|GetWidgets) _array_index _returnvalue true)
    (Widget|SetVisibility _returnvalue "Collapsed"))
  (CallFunction|SwitchtoWidget))

(fn ConstructionScript)

(fn SwitchtoWidget
  (params (WindowIndex :type Integer))
  (bind _widgets (Variables|Default|GetWidgets))
  (if (not (and (== WindowIndex (Variables|Default|GetCurrentWidgetIndex)) (Utilities|Array|IsValidIndex _widgets WindowIndex)))
    (if (Utilities|Array|IsValidIndex _widgets (Variables|Default|GetCurrentWidgetIndex))
      (Widget|SetVisibility (Utilities|Array|Get(acopy) _widgets (Variables|Default|GetCurrentWidgetIndex)) "Collapsed")
      (else
        (bind _output_get (Variables|Default|SetCurrentWidgetIndex WindowIndex))
        (Widget|SetVisibility (Utilities|Array|Get(acopy) _widgets _output_get) "Visible")))))