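; BP_HUDBase is a base HUD that manages a set of screen widgets and shows one at a time by index.
; BeginPlay creates every class in WidgetsClasses, adds each to the viewport collapsed, then shows the starting widget and calls InitFunc.
; SwitchToWidget toggles visibility and shows the mouse cursor only while a valid widget is active.
; InitFunc and OnWindowChange are empty hooks for child Blueprints.
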(event EventBeginPlay
  ;[1 1 1] Begin
  (if (> (Utilities|Array|Length (Variables|Default|GetWidgetsClasses)) 0)
    (for (_array_element _array_index) (Variables|Default|GetWidgetsClasses)
      (bind _returnvalue (UserInterface|CreateWidget _array_element))
      (UserInterface|Viewport|AddtoViewport _returnvalue 0)
      (Utilities|Array|SetArrayElem (Variables|Default|GetWidgets) _array_index _returnvalue true)
      (Widget|SetVisibility _returnvalue "Collapsed"))
    (CallFunction|SwitchtoWidget (Variables|Default|GetStartingWidgetIndex))
    (CallFunction|InitFunc)))

(fn ConstructionScript)

(fn SwitchtoWidget
  (params (WindowIndex :type Integer))
  (bind _widgets (Variables|Default|GetWidgets))
  (bind _widgets_2 (Variables|Default|GetWidgets))
  (if (not (== (Variables|Default|GetCurrentWidgetIndex) WindowIndex))
    (Utilities|FlowControl|Sequence
      (:then_0
        (if (Utilities|Array|IsValidIndex _widgets_2 (Variables|Default|GetCurrentWidgetIndex))
          (Widget|SetVisibility (Utilities|Array|Get(acopy) _widgets_2 (Variables|Default|GetCurrentWidgetIndex)) "Collapsed")
          (Variables|Default|SetIsUIActive false)))
      (:then_1
        (bind _output_get (Variables|Default|SetCurrentWidgetIndex WindowIndex))
        (if (Utilities|Array|IsValidIndex _widgets WindowIndex)
          (Widget|SetVisibility (Utilities|Array|Get(acopy) _widgets _output_get) "Visible")
          (Variables|Default|SetIsUIActive true)))
      (:then_2
        (Variables|/Script/Engine.PlayerController|SetbShowMouseCursor (Game|GetPlayerController 0) (Variables|Default|GetIsUIActive))
        (CallFunction|OnWindowChange)))))

(fn InitFunc)

(fn OnWindowChange)