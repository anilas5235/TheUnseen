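; BP_UnseenHUD is a HUD Blueprint that manages the player stats display and the game over screen.
; InitFunc creates the player stats widget and adds it to the viewport before calling the parent version.
; OnWindowChange hides the stats and switches to UI-only input while UI is active, restores both otherwise, then calls the parent.
; The GameOverScreen event removes all widgets and shows the game over widget.
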(event Custom|GameOverScreen
  (Viewport|RemoveAllWidgets)
  (bind _returnvalue (UserInterface|CreateWidget "/Game/Project/BluePrints/GUI/Transitions/WBP_GameOver.WBP_GameOver_C"))
  (UserInterface|Viewport|AddtoViewport _returnvalue 0))

(fn ConstructionScript)

(fn InitFunc
  (bind _returnvalue (UserInterface|CreateWidget "/Game/Project/BluePrints/GUI/InGame/WBP_PlayerStats.WBP_PlayerStats_C"))
  (bind _output_get (Variables|Default|SetPlayerStats _returnvalue))
  (UserInterface|Viewport|AddtoViewport _output_get 0)
  (|CallParentFunction))

(fn OnWindowChange
  (bind _returnvalue (Game|GetPlayerController 0))
  (bind _playerstats (Variables|Default|GetPlayerStats))
  (if (Variables|Default|GetIsUIActive)
    (Widget|SetVisibility _playerstats "Collapsed")
    (Input|SetInputModeUIOnly _returnvalue 0 "DoNotLock" false)
    (else
      (Widget|SetVisibility _playerstats "Visible")
      (Input|SetInputModeGameOnly _returnvalue false)))
  (|CallParentFunction))