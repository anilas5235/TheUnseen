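; BP_LightLamp is a lamp actor that tells the player controller when the Severog player character steps into or out of its light.
; A capsule's overlap events call PassedIntoLight and PassedOutofLight on BP_UnseenPlayerController.
; DisableLight and EnableLight toggle the spot light, point light and mesh visibility along with capsule overlap generation.
; If Flikering is set, a looping timer switches the lamp off for OutDuration, then back on.
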(event OnComponentBeginOverlap(Capsule)
  (params (OverlappedComponent :type Primitive%20Component%20Object%20Reference) (OtherActor :type Actor%20Object%20Reference) (OtherComp :type Primitive%20Component%20Object%20Reference) (OtherBodyIndex :type Integer) (bFromSweep :type Boolean) (SweepResult :type Hit%20Result%20Structure%20%28by%20ref%29))
  (bind _assevarog_player_character (Utilities|Casting|CastToSevarogPlayerCharacter OtherActor))
  (bind _asbp_unseen_player_controller (Utilities|Casting|CastToBP_UnseenPlayerController (Pawn|GetController _assevarog_player_character)))
  (Default|PassedIntoLight _asbp_unseen_player_controller self))

(event OnComponentEndOverlap(Capsule)
  (params (OverlappedComponent :type Primitive%20Component%20Object%20Reference) (OtherActor :type Actor%20Object%20Reference) (OtherComp :type Primitive%20Component%20Object%20Reference) (OtherBodyIndex :type Integer))
  (bind _assevarog_player_character (Utilities|Casting|CastToSevarogPlayerCharacter OtherActor))
  (bind _asbp_unseen_player_controller (Utilities|Casting|CastToBP_UnseenPlayerController (Pawn|GetController _assevarog_player_character)))
  (Default|PassedOutofLight _asbp_unseen_player_controller self))

(event Custom|Fliker
  (CallFunction|DisableLight)
  (Utilities|FlowControl|Delay (Variables|Default|GetOutDuration))
  (CallFunction|EnableLight))

(event EventBeginPlay
  (if (Variables|Default|GetFlikering)
    (Utilities|Time|SetTimerbyEvent (delegate Custom|Fliker) (Variables|Default|GetDelay) true)))

(fn ConstructionScript)

(fn DisableLight
  (if (Variables|Default|GetLightEnabled)
    (Variables|Default|SetLightEnabled false)
    (Development|SetHiddeninGame (Variables|Default|GetSpotLight) true false)
    (Variables|/Script/Engine.PrimitiveComponent|SetbGenerateOverlapEvents (Variables|Default|GetCapsule) false)))

(fn EnableLight
  (if (not (Variables|Default|GetLightEnabled))
    (Variables|Default|SetLightEnabled true)
    (Development|SetHiddeninGame (Variables|Default|GetSpotLight) false false)
    (Variables|/Script/Engine.PrimitiveComponent|SetbGenerateOverlapEvents (Variables|Default|GetCapsule) true)))