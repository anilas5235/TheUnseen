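; Player controller for a ghost that possesses objects, managing HP, energy, soul shards and game end.
; Possession swaps pawns on a cooldown, with a capsule trace checking room before returning to the ghost.
; Tick drains energy, then HP, while possessing; otherwise it regenerates energy and applies stacking light damage.
; Death or collecting all shards triggers game over, inserting a computed score into the saved leaderboard and showing it on the HUD.
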(event Custom|Start%20Posses%20Cooldown
  ;[1 1 1] posses cooldown
  (Variables|Default|SetCanPosses false)
  (Utilities|FlowControl|Delay (Variables|Default|GetPossesCoolDown))
  (Variables|Default|SetCanPosses true))

(event Custom|InitBars
  ;[1 1 1] Init Bars
  (Variables|Default|SetcurrentHP (Math|Conversions|ToFloat(Integer) (Variables|Default|GetmaxHP)))
  (CallFunction|UpdateHPVisual)
  (Variables|Default|SetcurrentEnergy (Math|Conversions|ToFloat(Integer) (Variables|Default|GetmaxEnergy)))
  (CallFunction|UpdateEnergyVisual))

(event Custom|GameOver
  ;[1 1 1] Game Over
  (Utilities|FlowControl|Sequence
    (:then_0
      (bind _assevarog_player_character (Utilities|Casting|CastToSevarogPlayerCharacter (Variables|Default|GetGhostCharacter)))
      (Default|DisableTrail _assevarog_player_character))
    (:then_1
      (bind _scorestruct (CallFunction|SaveScore))
      (bind _asbp_unseen_hud (CallFunction|TryGetUnseenHUD))
      (Default|GameOverScreen _asbp_unseen_hud _scorestruct (Variables|Default|GetEnding%20Type))
      (Actor|Tick|SetActorTickEnabled false))))

(event Custom|VisitedNewObj
  ;[1 1 1] visited new obj
  (Math|Integer|IncrementInt (Variables|Default|GetNumVisitedObjects)))

(event EventBeginPlay
  (bind _self self)
  (bind _returnvalue (PlayerController|LocalPlayerSubsystems|GetEnhancedInputLocalPlayerSubsystem _self))
  ;[1 1 1] Add Mapping
  (Class|EnhancedInputSubsystemInterface|ClearAllMappings _returnvalue)
  (Input|AddMappingContext _returnvalue "/Game/Project/Input/IMC_Unseen3Person.IMC_Unseen3Person" 0 "(bIgnoreAllPressedKeysUntilRelease=True,bForceImmediately=False,bNotifyUserSettings=False)")
  (Variables|Default|SetStartTime (Math|DateTime|UTCNow))
  (Input|SetInputModeGameOnly self false))

(event EventTick
  (params (DeltaSeconds :type Float%20%28single-precision%29))
  (bind _lights (Variables|Default|GetLights))
  (bind _returnvalue (Utilities|Set|Length _lights))
  (bind _returnvalue_2 (> _returnvalue 0))
  ;[1 1 1] Tick
  (if (> (Variables|Default|GetcurrentHP) 0.0)
    (if (Variables|Default|GetIsPossessingObj)
      (if (> (Variables|Default|GetcurrentEnergy) 0.0)
        ;;[1 1 1] Energy Drain
        (Variables|Default|SetcurrentEnergy (- (Variables|Default|GetcurrentEnergy) (* (Variables|Default|GetEnergyDeplitionRate) DeltaSeconds)))
        (CallFunction|UpdateEnergyVisual :!label _label)
        (else
          ;;[1 1 1] HP Drain
          (Variables|Default|SetcurrentHP (- (Variables|Default|GetcurrentHP) (* (Variables|Default|GetHPDeplitionRate) DeltaSeconds)))
          (CallFunction|UpdateHPVisual)))
      (else
        (Utilities|FlowControl|Sequence
          (:then_0
            (if (< (Variables|Default|GetcurrentEnergy) (Variables|Default|GetmaxEnergy))
              ;;[1 1 1] Energy Regen
              (Variables|Default|SetcurrentEnergy (+ (Variables|Default|GetcurrentEnergy) (* (Variables|Default|GetEnergyRegenRate) DeltaSeconds)))
              (goto _label)))
          (:then_1
            ;;[1 1 1] Is in Light ?
            (if (not (== (Variables|Default|GetIsInLight) _returnvalue_2))
              (bind _output_get (Variables|Default|SetIsInLight _returnvalue_2))
              (bind _assevarog_player_character (Utilities|Casting|CastToSevarogPlayerCharacter (Variables|Default|GetGhostCharacter)))
              (if _output_get
                (Default|EnableTrail _assevarog_player_character)
                (else
                  (Default|DisableTrail _assevarog_player_character)))))
          (:then_2
            (if (Variables|Default|GetIsInLight)
              ;;[1 1 1] Light HP penelty
              (Variables|Default|SetcurrentHP (- (Variables|Default|GetcurrentHP) (* (* (Variables|Default|GetHPDeplitionRate) DeltaSeconds) (+ (* (- _returnvalue 1) 0.2) (Variables|Default|GetLightPeneltyMultiplier)))))
              (CallFunction|UpdateHPVisual))))))
    (else
      (Variables|Default|SetEnding%20Type "NewEnumerator0")
      (CallFunction|GameOver))))

(fn ConstructionScript)

(fn PossesObj
  (params (TargetPawn :type BP%20Possessable%20Object%20Object%20Reference))
  (if (Variables|Default|GetCanPosses)
    (Pawn|Possess self TargetPawn)
    (Transformation|SetWorldRotation (Variables|/Game/Project/BluePrints/BP_PossessableObject.BP_PossessableObject_C|GetSpringArm TargetPawn) (Transformation|GetWorldRotation (Variables|/Script/Engine.Character|GetCapsuleComponent (Variables|Default|GetGhostCharacter))) false false)
    (Variables|Default|SetIsPossessingObj true)
    (CallFunction|StartPossesCooldown)))

(fn PossesGhost
  (params (NewLocation :type Vector) (NewRotation :type Rotator))
  (bind _ghostcharacter (Variables|Default|GetGhostCharacter))
  (bind _ghostcharacter_2 (Variables|Default|GetGhostCharacter))
  (bind _capsulecomponent (Variables|/Script/Engine.Character|GetCapsuleComponent _ghostcharacter_2))
  (bind _returnvalue (Components|Capsule|GetScaledCapsuleHalfHeight _capsulecomponent))
  (bind _returnvalue_2 (+ NewLocation (Math|Vector|MakeVector 0.0 0.0 _returnvalue)))
  (if (Variables|Default|GetCanPosses)
    (bind _returnvalue_3 (Class|KismetSystemLibrary|CapsuleTraceSingleforObjects _returnvalue_2 _returnvalue_2 (Components|Capsule|GetScaledCapsuleRadius _capsulecomponent) _returnvalue (Utilities|Array|MakeArray "ObjectTypeQuery1" "ObjectTypeQuery3" "ObjectTypeQuery2") false (Utilities|Array|MakeArray _ghostcharacter_2) "ForDuration" true))
    (if (not _returnvalue_3)
      (Transformation|SetActorLocationAndRotation _ghostcharacter _returnvalue_2 NewRotation false true)
      (Pawn|Possess self _ghostcharacter)
      (CallFunction|StartPossesCooldown)
      (Variables|Default|SetIsPossessingObj false))))

(fn UpdateEnergyVisual
  (bind _asbp_unseen_hud (CallFunction|TryGetUnseenHUD))
  (Default|UpdateEnergyBar (Variables|/Game/Project/BluePrints/GUI/HUDs/BP_UnseenHUD.BP_UnseenHUD_C|GetPlayerStats _asbp_unseen_hud) (/ (Variables|Default|GetcurrentEnergy) (Variables|Default|GetmaxEnergy))))

(fn UpdateHPVisual
  (bind _asbp_unseen_hud (CallFunction|TryGetUnseenHUD))
  (Default|UpdateHPBar (Variables|/Game/Project/BluePrints/GUI/HUDs/BP_UnseenHUD.BP_UnseenHUD_C|GetPlayerStats _asbp_unseen_hud) (/ (Variables|Default|GetcurrentHP) (Variables|Default|GetmaxHP))))

(fn PassedIntoLight
  (params (LightActor :type Actor%20Object%20Reference%20%28by%20ref%29))
  (Utilities|Set|Add (Variables|Default|GetLights) LightActor))

(fn PassedOutofLight
  (params (LightActor :type Actor%20Object%20Reference%20%28by%20ref%29))
  (Utilities|Set|Remove (Variables|Default|GetLights) LightActor))

(fn SaveScore
  (bind _returnvalue (Math|DateTime|UTCNow))
  (bind _maxhp (Variables|Default|GetmaxHP))
  (bind _currenthp (Variables|Default|GetcurrentHP))
  (bind _starttime (Variables|Default|GetStartTime))
  (bind _numvisitedobjects (Variables|Default|GetNumVisitedObjects))
  (bind _soulshards (Variables|Default|GetSoulShards))
  (bind _returnvalue_2 (- _returnvalue _starttime))
  (bind _returnvalue_3 (Math|Conversions|ToFloat(Integer) _maxhp))
  (bind _returnvalue_4 (* _numvisitedobjects 100))
  (bind _returnvalue_5 (* (.x _soulshards) 500))
  (bind _returnvalue_6 (Class|KismetMathLibrary|GetTotalMilliseconds _returnvalue_2))
  (bind _returnvalue_7 (Math|Float|Clamp(Float) _currenthp 0.0 _returnvalue_3))
  (bind _returnvalue_8 (/ _returnvalue_6 1e+03))
  (bind _returnvalue_9 (/ _returnvalue_7 _maxhp))
  (bind _returnvalue_10 (* _returnvalue_9 1e+02))
  (bind _returnvalue_11 (* _returnvalue_10 5e+01))
  (bind _returnvalue_12 (+ _returnvalue_4 _returnvalue_11 _returnvalue_5))
  (bind _returnvalue_13 (- _returnvalue_12 _returnvalue_8))
  (bind _returnvalue_14 (Math|Float|Truncate _returnvalue_13))
  (bind _s_unseenscore (Utilities|Struct|MakeS_UnseenScore _returnvalue_14 _returnvalue_8 _numvisitedobjects _returnvalue_10 (.x _soulshards)))
  (bind __score_save (CallFunction|GetScoreSave))
  (bind (_array_element _array_index) (Utilities|Array|ForEachLoopwithBreak (Variables|/Game/Project/CustomDataTypes/Saves/SG_ScoreSave.SG_ScoreSave_C|GetScoreBoard __score_save) :!label _label)
    (:LoopBody
      (if (< (.TotalScore (Utilities|Struct|BreakS_UnseenScore _array_element)) (.TotalScore (Utilities|Struct|BreakS_UnseenScore _s_unseenscore)))
        (Utilities|Array|Insert (Variables|/Game/Project/CustomDataTypes/Saves/SG_ScoreSave.SG_ScoreSave_C|GetScoreBoard __score_save) _s_unseenscore _array_index)
        (LocalVariables|SetputInList true)
        (goto _label Break)))
    (:Completed
      (if (LocalVariables|GetputInList)
        _
        (else
          (Utilities|Array|Add (Variables|/Game/Project/CustomDataTypes/Saves/SG_ScoreSave.SG_ScoreSave_C|GetScoreBoard __score_save) _s_unseenscore)))
      (CallFunction|SaveScoreSave __score_save)
      (return (|Copy _s_unseenscore)))))

(fn Collected
  (params (Type :type E_Collectables%20Enum :default "NewEnumerator0"))
  (bind _soulshards (Variables|Default|GetSoulShards))
  (switch Utilities|FlowControl|Switch|SwitchonE_Collectables Type
    (:NewEnumerator0
      (bind _result (Math|Integer|IncrementInt (.x _soulshards))
        (:%20%20
          (Utilities|FlowControl|Sequence
            (:then_0
              (bind _asbp_unseen_hud (CallFunction|TryGetUnseenHUD))
              (Default|UpdateSoulShards (Variables|/Game/Project/BluePrints/GUI/HUDs/BP_UnseenHUD.BP_UnseenHUD_C|GetPlayerStats _asbp_unseen_hud)))
            (:then_1
              (if (>= _result (.y _soulshards))
                (Variables|Default|SetEnding%20Type "NewEnumerator1")
                (CallFunction|GameOver)))))))))

(fn AddNumberOfCollectable
  (params (Type :type E_Collectables%20Enum :default "NewEnumerator0"))
  (switch Utilities|FlowControl|Switch|SwitchonE_Collectables Type
    (:NewEnumerator0
      (Math|Integer|IncrementInt (.y (Variables|Default|GetSoulShards))))))